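; NPC actor that shows dialogue in a widget component and completes the player's quest when the conversation ends.
; Each Talk call flags the OnGroundPawn as talking, hides the quest indicator and displays the next Dialogue line in the cached WB_Dialogue.
; Past the last line it hides the dialogue, marks the pawn done and calls CompleteQuest through a DoOnce.
; A sound node for voice or music is left unconnected.
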(event `self.ReceiveBeginPlay`
  (bind _dialoguewidget (`self.DialogueWidget`))
  ;[1 1 1] Assign the widget component to the UI
  (`SceneComponent.SetVisibility` _dialoguewidget false false)
  (bind _aswb_dialogue (cast `/Game/Blueprints/NPC/Dialogue/WB_Dialogue` (`WidgetComponent.GetUserWidgetObject` _dialoguewidget)))
  (set `self.UI` _aswb_dialogue))

(event `/Game/Blueprints/NPC/Dialogue/BPI_Dialogue.Talk`
  ;[1 1 1] NPC Dialogue Controller
  (bind _ason_ground_pawn (cast `/Game/Blueprints/Movment/OnGroundPawn` (`GameplayStatics.GetPlayerPawn` 0)))
  (set `/Game/Blueprints/Movment/OnGroundPawn.isTalking` true _ason_ground_pawn)
  (`/Engine/EditorBlueprintResources/StandardMacros.IncrementInt` (`self.talkIndex`)
    (:`  `
      (if (< (`self.talkIndex`) (`KismetArrayLibrary.Array_Length` (`self.dialogue`)))
        (`self.UI`
          (:`then`
            _)
          (:`else`
            (bind _returnvalue (`|CreateWidget` "/Game/Blueprints/NPC/Dialogue/WB_Dialogue.WB_Dialogue_C" (`GameplayStatics.GetPlayerController` 0)))
            (set `self.UI` _returnvalue)))
        (`TextBlock.SetText` (`/Game/Blueprints/NPC/Dialogue/WB_Dialogue.TalkText` (`self.UI`)) (`KismetTextLibrary.Conv_StringToText` (`|GetArrayItem` (`self.dialogue`) (`self.talkIndex`))))
        (`SceneComponent.SetVisibility` (`self.DialogueWidget`) true false)
        (`SceneComponent.SetVisibility` (`self.quest indicator`) false false)
        (else
          (`Widget.RemoveFromParent` (`self.UI`))
          (bind _ason_ground_pawn_2 (cast `/Game/Blueprints/Movment/OnGroundPawn` (`GameplayStatics.GetPlayerPawn` 0)))
          (set `/Game/Blueprints/Movment/OnGroundPawn.isTalking` false _ason_ground_pawn_2)
          (set `/Game/Blueprints/Movment/OnGroundPawn.isDone` true _ason_ground_pawn_2)
          (`SceneComponent.SetVisibility` (`self.DialogueWidget`) false false)
          (`/Engine/EditorBlueprintResources/StandardMacros.DoOnce` false
            (:`Completed`
              (`/Game/Blueprints/Movment/OnGroundPawn.CompleteQuest` _ason_ground_pawn_2))))))))

(fn `UserConstructionScript`)