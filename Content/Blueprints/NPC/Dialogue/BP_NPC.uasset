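; NPC Blueprint for dialogue and random roaming, with much of its logic left disconnected.
; Talk advances through the Dialogue array; past the end, it removes the UI, updates the Joystick actor's talk flags and completes its quest once.
; The widget display, which flags VRPawnTEST as talking, and the sound playback are unwired.
; Roam loops AI moves to random reachable nearby points, but its starting call is also unwired.
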(event `self.ReceiveBeginPlay`
  ;[1 1 1] AI Roam Around (Random roam)
)

(event `Roam`
  ;[1 1 1] AI Roam Around (Random roam)
  (`|AIMoveTo` self (`NavigationSystemV1.K2_GetRandomReachablePointInRadius` (`self.K2_GetActorLocation`) 2000.0 null null) null
    (:`OnSuccess`
      (`self.Roam`))))

(event `self.Talk`
  ;[1 1 1] NPC Dialogue Controller
  (`/Engine/EditorBlueprintResources/StandardMacros.IncrementInt` (`self.talkIndex`)
    (:`  `
      (if (not (< (`self.talkIndex`) (`KismetArrayLibrary.Array_Length` (`self.dialogue`))))
        (`Widget.RemoveFromParent` (`self.UI`))
        (bind _returnvalue (`GameplayStatics.GetActorOfClass` "/Game/Blueprints/Movment/joystick.joystick_C"))
        (set `/Game/Blueprints/Movment/joystick.isTalking` false _returnvalue)
        (set `/Game/Blueprints/Movment/joystick.isDone` true _returnvalue)
        (`/Engine/EditorBlueprintResources/StandardMacros.DoOnce` false
          (:`Completed`
            (`/Game/Blueprints/Movment/joystick.CompleteQuest` _returnvalue)))))))

(fn `UserConstructionScript`)