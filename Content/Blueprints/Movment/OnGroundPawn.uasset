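; VR ground pawn that the player walks around in to talk to NPCs, follow quests and swap bodies.
; Thumbsticks drive camera-relative movement and snap turning, while buttons trigger BPI_Dialogue on overlapping NPCs, next-pawn possession via PC_possesion, or an in-world menu.
; A Paused flag blocks walking during menus and dialogue and enables trigger clicks through widget interaction components, with spline-mesh pointers rebuilt every tick.
; A viewport widget shows the current mission text.
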(event `InputAction|ButtonX`
  (params (Key :type "Key Structure"))
  (bind _overlappingactors (`self.GetOverlappingActors` "/Game/Blueprints/NPC/Dialogue/BP_NPC1.BP_NPC1_C"))
  ;[1 1 1] Quest
  ;;[1 1 1] Overlapping with NPC Dialogue system
  (:`Pressed`
    (if (> (`KismetArrayLibrary.Array_Length` _overlappingactors) 0)
      (set `self.Paused` true)
      (for _array_element _overlappingactors
        (if (`KismetSystemLibrary.DoesImplementInterface` _array_element "/Game/Blueprints/NPC/Dialogue/BPI_Dialogue.BPI_Dialogue_C")
          (message `/Game/Blueprints/NPC/Dialogue/BPI_Dialogue.Talk` _array_element)
          (if (not (`self.isTalking`))
            (set `self.Paused` false)))))))

(event `CompleteQuest`
  ;[1 1 1] Quest
  ;;[1 1 1] Complete quest
  (if (`self.isDone`)
    (bind _output_get (set `self.currentMission` "QUEST COMPLETE"))
    (`self.UpdateMission` _output_get)
    (set `self.isDone` false)))

(event `QuestUI`
  ;[1 1 1] Quest
  ;;[1 1 1] Quest/mission UI
  (bind _returnvalue (`|CreateWidget` "/Game/Blueprints/NPC/Quest/WP_Mission.WP_Mission_C" (`GameplayStatics.GetPlayerController` 0)))
  (bind _output_get (set `self.missionWidget` _returnvalue))
  (`UserWidget.AddToViewport` _output_get 0))

(event `self.ReceiveBeginPlay`
  ;[1 1 1] Movement
  (`HeadMountedDisplayFunctionLibrary.SetTrackingOrigin` "Floor")
  (`self.QuestUI`)
  (bind _returnvalue (`|SpawnActorFromClass` "/Game/Blueprints/UI/InGameMenu/InGameMenuWidget.InGameMenuWidget_C" (`KismetMathLibrary.MakeTransform` (0.0 0.0 0.0)) "Undefined" "OverrideRootScale" null null))
  (bind _output_get (set `self.MenuWidget` _returnvalue))
  (`Widget.SetVisibility` (`WidgetComponent.GetWidget` (`/Game/Blueprints/UI/InGameMenu/InGameMenuWidget.Widget` _output_get)) "Hidden"))

(event `InputAxis|MovementAxisRight_X`
  (params (AxisValue :type "Float (single-precision)"))
  (bind (_returnvalue_x _returnvalue_y) (`KismetMathLibrary.BreakVector` (`SceneComponent.GetRightVector` (`self.Camera`))))
  ;[1 1 1] Movement
  (if (`self.Paused`)
    _
    (elif (not (== AxisValue 0.0))
      (`self.AddMovementInput` (`KismetMathLibrary.MakeVector` _returnvalue_x _returnvalue_y) (* AxisValue (`self.movment  speed`))))))

(event `InputAxis|MovementAxisRight_Y`
  (params (AxisValue :type "Float (single-precision)"))
  (bind (_returnvalue_x _returnvalue_y) (`KismetMathLibrary.BreakVector` (`SceneComponent.GetForwardVector` (`self.Camera`))))
  ;[1 1 1] Movement
  (if (`self.Paused`)
    _
    (elif (not (== AxisValue 0.0))
      (`self.AddMovementInput` (`KismetMathLibrary.MakeVector` _returnvalue_x _returnvalue_y) (* AxisValue (`self.movment  speed`))))))

(event `InputAxis|MovementAxisLeft_X`
  (params (AxisValue :type "Float (single-precision)"))
  (bind (_returnvalue_location _returnvalue_rotation _returnvalue_scale) (`KismetMathLibrary.BreakTransform` (`self.GetTransform`)))
  (bind (_returnvalue_roll _returnvalue_pitch _returnvalue_yaw) (`KismetMathLibrary.BreakRotator` (`self.K2_GetActorRotation`)))
  (bind _rotationdeadzone (`self.rotationDeadZone`))
  ;[1 1 1] Movement
  (if (== AxisValue 0.0)
    (goto _label :!via `Reset`)
    (elif (>= AxisValue _rotationdeadzone)
      (set `self.rotationAngle` 22.5)
      (`/Engine/EditorBlueprintResources/StandardMacros.DoOnce` false :!label _label
        (:`Completed`
          (`self.K2_SetActorTransform` (`KismetMathLibrary.MakeTransform` _returnvalue_location (`KismetMathLibrary.MakeRotator` 0.0 0.0 (+ _returnvalue_yaw (`self.rotationAngle`))) _returnvalue_scale))))
      (elif (<= AxisValue (* _rotationdeadzone -1.0))
        (set `self.rotationAngle` -22.5)
        (goto _label)
        (elif (or (> AxisValue -0.2) (< AxisValue 0.2))
          (goto _label :!via `Reset`))))))

(event `InputAction|ButtonA`
  (params (Key :type "Key Structure"))
  ;[1 1 1] bodyswap
  (:`Pressed`
    (if (not (`self.Paused`))
      (bind _aspc_possesion (cast `/Game/Blueprints/Movment/PC_possesion` (`GameplayStatics.GetPlayerController` 0)))
      (`/Game/Blueprints/Movment/PC_possesion.nextPlayerPosses` _aspc_possesion))))

(event `InputAction|ButtonB`
  (params (Key :type "Key Structure"))
  (bind (_returnvalue_location _returnvalue_rotation) (`KismetMathLibrary.BreakTransform` (`self.GetTransform`)))
  ;[1 1 1] IngameMenu Interaction
  (:`Pressed`
    (if (not (`self.Paused`))
      (set `self.Paused` true)
      (bind _menuwidget (`self.MenuWidget`)
        (:`then`
          (`Widget.SetVisibility` (`WidgetComponent.GetWidget` (`/Game/Blueprints/UI/InGameMenu/InGameMenuWidget.Widget` _menuwidget)) "Visible")
          (`self.K2_SetActorTransform` _menuwidget (`KismetMathLibrary.MakeTransform` (+ (+ _returnvalue_location (0.0 0.0 100.0)) (* (`self.GetActorForwardVector`) (`KismetMathLibrary.Conv_DoubleToVector` 600.0))) (`KismetMathLibrary.ComposeRotators` _returnvalue_rotation (`KismetMathLibrary.MakeRotator` 0.0 0.0 180.0))) false false))
        (:`else`)))))

(event `self.ReceiveTick`
  (params (DeltaSeconds :type "Float (single-precision)"))
  ;[1 1 1] IngameMenu Interaction
  (`self.WidgetInteractionForIngame`))

(event `InputAction|TriggerLeft`
  (params (Key :type "Key Structure"))
  (bind _widgetinteractionleft (`self.WidgetInteractionLeft`))
  (bind _istalking (`self.isTalking`))
  (bind _paused (`self.Paused`))
  ;[1 1 1] IngameMenu Interaction
  (:`Pressed`
    (if _istalking
      _
      (elif _paused
        (`WidgetInteractionComponent.PressPointerKey` _widgetinteractionleft "LeftMouseButton"))))
  (:`Released`
    (if _istalking
      _
      (elif _paused
        (`WidgetInteractionComponent.ReleasePointerKey` _widgetinteractionleft "LeftMouseButton")
        (set `self.Paused` false :!label _label_2)))))

(event `InputAction|TriggerRight`
  (params (Key :type "Key Structure"))
  (bind _paused (`self.Paused`))
  (bind _widgetinteractionright (`self.WidgetInteractionRight`))
  (bind _istalking (`self.isTalking`))
  ;[1 1 1] IngameMenu Interaction
  (:`Pressed`
    (if _istalking
      _
      (elif _paused
        (`WidgetInteractionComponent.PressPointerKey` _widgetinteractionright "LeftMouseButton"))))
  (:`Released`
    (if _istalking
      _
      (elif _paused
        (`WidgetInteractionComponent.ReleasePointerKey` _widgetinteractionright "LeftMouseButton")
        (goto _label_2)))))

(fn `UpdateMission`
  (params (currentMission :type String))
  ;[1 1 1] Updates quest UI Text
  (set `self.currentMission` currentMission)
  (`TextBlock.SetText` (`/Game/Blueprints/NPC/Quest/WP_Mission.currentMissionText` (`self.missionWidget`)) (`KismetTextLibrary.Conv_StringToText` (`self.currentMission`))))

(fn `UserConstructionScript`)

(fn `WidgetInteractionForIngame`
  (bind _widgetinteractionleft (`self.WidgetInteractionLeft`))
  (bind _widgetinteractionright (`self.WidgetInteractionRight`))
  (bind _returnvalue (`SceneComponent.K2_GetComponentLocation` _widgetinteractionright))
  (bind _returnvalue_2 (`SceneComponent.K2_GetComponentLocation` _widgetinteractionleft))
  (bind (_returnvalue_bblockinghit _returnvalue_binitialoverlap _returnvalue_time _returnvalue_distance _returnvalue_location) (`GameplayStatics.BreakHitResult` (`WidgetInteractionComponent.GetLastHitResult` _widgetinteractionleft)))
  (bind (_returnvalue_bblockinghit_2 _returnvalue_binitialoverlap_2 _returnvalue_time_2 _returnvalue_distance_2 _returnvalue_location_2) (`GameplayStatics.BreakHitResult` (`WidgetInteractionComponent.GetLastHitResult` _widgetinteractionright)))
  (bind _returnvalue_3 (`KismetMathLibrary.GetForwardVector` (`KismetMathLibrary.FindLookAtRotation` _returnvalue_2 _returnvalue_location)))
  (bind _returnvalue_4 (`KismetMathLibrary.GetForwardVector` (`KismetMathLibrary.FindLookAtRotation` _returnvalue _returnvalue_location_2)))
  (`|ExecutionSequence`
    (:`then_0`
      (bind _leftspline (`self.LeftSpline`)
        (:`then`
          (`ActorComponent.K2_DestroyComponent` _leftspline))
        (:`else`
          _))
      (if (`WidgetInteractionComponent.IsOverHitTestVisibleWidget` _widgetinteractionleft)
        (bind _returnvalue_5 (`AddComponent|NODE_AddSplineMeshComponent-0` :`bManualAttachment` true))
        (bind _output_get (set `self.LeftSpline` _returnvalue_5))
        (`SplineMeshComponent.SetStartAndEnd` _output_get _returnvalue_2 _returnvalue_3 _returnvalue_location (* _returnvalue_3 (`KismetMathLibrary.Conv_DoubleToVector` -1.0)) true)))
    (:`then_1`
      (bind _rightspline (`self.RightSpline`)
        (:`then`
          (`ActorComponent.K2_DestroyComponent` _rightspline))
        (:`else`
          _))
      (if (`WidgetInteractionComponent.IsOverHitTestVisibleWidget` _widgetinteractionright)
        (bind _returnvalue_6 (`AddComponent|NODE_AddSplineMeshComponent-1` :`bManualAttachment` true))
        (bind _output_get_2 (set `self.RightSpline` _returnvalue_6))
        (`SplineMeshComponent.SetStartAndEnd` _output_get_2 _returnvalue _returnvalue_4 _returnvalue_location_2 (* _returnvalue_4 (`KismetMathLibrary.Conv_DoubleToVector` -1.0)) true)))))