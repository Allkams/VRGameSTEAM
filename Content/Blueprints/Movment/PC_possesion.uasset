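; Player controller Blueprint that hands control between the Joystick pawns placed in the level.
; On BeginPlay it finds all Joystick actors and possesses the first one.
; The nextPlayerPosses event fetches the list again, advances CurrentPlayerIndex with wraparound to zero, and possesses the pawn at that index.
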(event `self.ReceiveBeginPlay`
  (bind _outactors (`GameplayStatics.GetAllActorsOfClass` "/Game/Blueprints/Movment/joystick.joystick_C"))
  (bind _aspawn (cast `Pawn` (`|GetArrayItem` _outactors)))
  (`self.Possess` _aspawn))

(event `nextPlayerPosses`
  (bind _returnvalue (+ (`self.currentPlayerIndex`) 1))
  (bind _outactors (`GameplayStatics.GetAllActorsOfClass` "/Game/Blueprints/Movment/joystick.joystick_C"))
  (if (== (`KismetArrayLibrary.Array_Length` _outactors) _returnvalue)
    (set `self.currentPlayerIndex` 0)
    (else
      (set `self.currentPlayerIndex` _returnvalue)))
  (bind _aspawn (cast `Pawn` (`|GetArrayItem` _outactors (`self.currentPlayerIndex`))))
  (`self.Possess` _aspawn))

(fn `UserConstructionScript`)