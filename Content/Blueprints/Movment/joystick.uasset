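; VR player pawn with joystick locomotion, NPC dialogue, quest display and body swapping.
; Right-stick axes drive camera-relative horizontal movement, while left-stick X sets up 45-degree snap turns gated by a dead zone and DoOnce.
; An Oculus face button sends TalkMessage to overlapping NPCs through BPI_Dialogue, and either trigger asks PC_possesion to possess the next body.
; A mission widget created at BeginPlay shows quest text, updated on quest completion.
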(event `InputAxisKey|OculusTouch_Left_FaceButton1`
  (params (AxisValue :type "Float (single-precision)"))
  ;[1 1 1] Overlapping with NPC Dialogue system
  (for _array_element (`self.GetOverlappingActors` "/Game/Blueprints/NPC/Dialogue/BP_NPC.BP_NPC_C")
    (if (`KismetSystemLibrary.DoesImplementInterface` _array_element "/Game/Blueprints/NPC/Dialogue/BPI_Dialogue.BPI_Dialogue_C")
      (message `/Game/Blueprints/NPC/Dialogue/BPI_Dialogue.Talk` _array_element)
      (if (`self.isTalking`)
        (`KismetSystemLibrary.PrintString` "Condition met")
        (else
          (`KismetSystemLibrary.PrintString` "Condition not met"))))))

(event `CompleteQuest`
  ;[1 1 1] Complete quest
  (if (`self.isDone`)
    (bind _output_get (set `self.currentMission` "QUEST COMPLETE"))
    (`self.UpdateMission` _output_get)
    (set `self.isDone` false)))

(event `self.ReceiveBeginPlay`
  (`HeadMountedDisplayFunctionLibrary.SetTrackingOrigin` "Floor")
  (`self.QuestUI`))

(event `QuestUI`
  ;[1 1 1] Quest/mission UI
  (bind _returnvalue (`|CreateWidget` "/Game/Blueprints/NPC/Quest/WP_Mission.WP_Mission_C" (`GameplayStatics.GetPlayerController` 0)))
  (bind _output_get (set `self.missionWidget` _returnvalue))
  (`UserWidget.AddToViewport` _output_get 0))

(event `InputAxis|MovementAxisRight_X`
  (params (AxisValue :type "Float (single-precision)"))
  (bind (_returnvalue_x _returnvalue_y) (`KismetMathLibrary.BreakVector` (`SceneComponent.GetRightVector` (`self.Camera`))))
  (if (not (== AxisValue 0.0))
    (`self.AddMovementInput` (`KismetMathLibrary.MakeVector` _returnvalue_x _returnvalue_y) (* AxisValue (`self.movment  speed`)))))

(event `InputAxis|MovementAxisRight_Y`
  (params (AxisValue :type "Float (single-precision)"))
  (bind (_returnvalue_x _returnvalue_y) (`KismetMathLibrary.BreakVector` (`SceneComponent.GetForwardVector` (`self.Camera`))))
  (if (not (== AxisValue 0.0))
    (`self.AddMovementInput` (`KismetMathLibrary.MakeVector` _returnvalue_x _returnvalue_y) (* AxisValue (`self.movment  speed`)))))

(event `InputAxis|MovementAxisLeft_X`
  (params (AxisValue :type "Float (single-precision)"))
  (bind (_returnvalue_location _returnvalue_rotation _returnvalue_scale) (`KismetMathLibrary.BreakTransform` (`self.GetTransform`)))
  (bind (_returnvalue_roll _returnvalue_pitch _returnvalue_yaw) (`KismetMathLibrary.BreakRotator` (`self.K2_GetActorRotation`)))
  (bind _rotationdeadzone (`self.rotationDeadZone`))
  (if (== AxisValue 0.0)
    (goto _label :!via `Reset`)
    (elif (>= AxisValue _rotationdeadzone)
      (set `self.rotationAngle` 45.0)
      (`/Engine/EditorBlueprintResources/StandardMacros.DoOnce` false :!label _label
        (:`Completed`
          (`self.K2_SetActorTransform` (`KismetMathLibrary.MakeTransform` _returnvalue_location (`KismetMathLibrary.MakeRotator` 0.0 0.0 (+ _returnvalue_yaw (`self.rotationAngle`))) _returnvalue_scale))))
      (elif (<= AxisValue (* _rotationdeadzone -1.0))
        (set `self.rotationAngle` -45.0)
        (goto _label)
        (elif (or (> AxisValue -0.2) (< AxisValue 0.2))
          (goto _label :!via `Reset`))))))

(event `InputAction|TriggerLeft`
  (params (Key :type "Key Structure"))
  ;[1 1 1] bodyswap (cant change motion sorcce ????)
  (:`Pressed`
    (bind _aspc_possesion (cast `/Game/Blueprints/Movment/PC_possesion` (`GameplayStatics.GetPlayerController` 0) :!label _label_2))
    (`/Game/Blueprints/Movment/PC_possesion.nextPlayerPosses` _aspc_possesion)))

(event `InputAction|TriggerRight`
  (params (Key :type "Key Structure"))
  ;[1 1 1] bodyswap (cant change motion sorcce ????)
  (:`Pressed`
    (goto _label_2)))

(event `self.ReceivePossessed`
  (params (NewController :type "Controller Object Reference"))
  ;[1 1 1] bodyswap (cant change motion sorcce ????)
)

(fn `UpdateMission`
  (params (currentMission :type String))
  ;[1 1 1] Updates quest UI Text
  (set `self.currentMission` currentMission)
  (`TextBlock.SetText` (`/Game/Blueprints/NPC/Quest/WP_Mission.currentMissionText` (`self.missionWidget`)) (`KismetTextLibrary.Conv_StringToText` (`self.currentMission`))))

(fn `UserConstructionScript`)