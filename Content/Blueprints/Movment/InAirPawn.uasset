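; VR pawn for in-air play, with stick movement along the horizontal plane, 22.5-degree snap turning and possession swapping through PC_possesion.
; Button B sets a paused flag and shows a world-space menu, clicked with trigger-driven widget interaction and spline lasers rebuilt each tick.
; An attached, elongated pointer actor highlights grid blocks through overlap events.
; Right-trigger presses alternate between spawning a house attached to the selected block and destroying its attached actor.
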(event `self.ReceiveBeginPlay`
  ;[1 1 1] Movement
  (`HeadMountedDisplayFunctionLibrary.SetTrackingOrigin` "Floor")
  (bind _returnvalue (`|SpawnActorFromClass` "/Game/Blueprints/UI/InGameMenu/InGameMenuWidget.InGameMenuWidget_C" (`KismetMathLibrary.MakeTransform` (0.0 0.0 0.0)) "Undefined" "OverrideRootScale" null null))
  (bind _output_get (set `self.MenuWidget` _returnvalue))
  (`Widget.SetVisibility` (`WidgetComponent.GetWidget` (`/Game/Blueprints/UI/InGameMenu/InGameMenuWidget.Widget` _output_get)) "Hidden")
  (`self.SetupGridPointer`))

(event `InputAxis|MovementAxisRight_X`
  (params (AxisValue :type "Float (single-precision)"))
  (bind (_returnvalue_x _returnvalue_y) (`KismetMathLibrary.BreakVector` (`SceneComponent.GetRightVector` (`self.Camera`))))
  ;[1 1 1] Movement
  (if (`self.Paused`)
    _
    (elif (not (== AxisValue 0.0))
      (`self.AddMovementInput` (`KismetMathLibrary.MakeVector` _returnvalue_x _returnvalue_y) (* AxisValue (`self.movment  speed`))))))

(event `InputAxis|MovementAxisRight_Y`
  (params (AxisValue :type "Float (single-precision)"))
  (bind (_returnvalue_x _returnvalue_y) (`KismetMathLibrary.BreakVector` (`SceneComponent.GetForwardVector` (`self.Camera`))))
  ;[1 1 1] Movement
  (if (`self.Paused`)
    _
    (elif (not (== AxisValue 0.0))
      (`self.AddMovementInput` (`KismetMathLibrary.MakeVector` _returnvalue_x _returnvalue_y) (* AxisValue (`self.movment  speed`))))))

(event `InputAxis|MovementAxisLeft_X`
  (params (AxisValue :type "Float (single-precision)"))
  (bind (_returnvalue_location _returnvalue_rotation _returnvalue_scale) (`KismetMathLibrary.BreakTransform` (`self.GetTransform`)))
  (bind (_returnvalue_roll _returnvalue_pitch _returnvalue_yaw) (`KismetMathLibrary.BreakRotator` (`self.K2_GetActorRotation`)))
  (bind _rotationdeadzone (`self.rotationDeadZone`))
  ;[1 1 1] Movement
  (if (== AxisValue 0.0)
    (goto _label :!via `Reset`)
    (elif (>= AxisValue _rotationdeadzone)
      (set `self.rotationAngle` 22.5)
      (`/Engine/EditorBlueprintResources/StandardMacros.DoOnce` false :!label _label
        (:`Completed`
          (`self.K2_SetActorTransform` (`KismetMathLibrary.MakeTransform` _returnvalue_location (`KismetMathLibrary.MakeRotator` 0.0 0.0 (+ _returnvalue_yaw (`self.rotationAngle`))) _returnvalue_scale))))
      (elif (<= AxisValue (* _rotationdeadzone -1.0))
        (set `self.rotationAngle` -22.5)
        (goto _label)
        (elif (or (> AxisValue -0.2) (< AxisValue 0.2))
          (goto _label :!via `Reset`))))))

(event `InputAction|ButtonA`
  (params (Key :type "Key Structure"))
  ;[1 1 1] bodyswap
  (:`Pressed`
    (if (not (`self.Paused`))
      (bind _aspc_possesion (cast `/Game/Blueprints/Movment/PC_possesion` (`GameplayStatics.GetPlayerController` 0)))
      (`/Game/Blueprints/Movment/PC_possesion.nextPlayerPosses` _aspc_possesion))))

(event `InputAction|ButtonB`
  (params (Key :type "Key Structure"))
  (bind (_returnvalue_location _returnvalue_rotation) (`KismetMathLibrary.BreakTransform` (`self.GetTransform`)))
  ;[1 1 1] IngameMenu Interaction
  (:`Pressed`
    (if (not (`self.Paused`))
      (set `self.Paused` true)
      (bind _menuwidget (`self.MenuWidget`)
        (:`then`
          (`Widget.SetVisibility` (`WidgetComponent.GetWidget` (`/Game/Blueprints/UI/InGameMenu/InGameMenuWidget.Widget` _menuwidget)) "Visible")
          (`self.K2_SetActorTransform` _menuwidget (`KismetMathLibrary.MakeTransform` (+ (+ _returnvalue_location (0.0 0.0 100.0)) (* (`self.GetActorForwardVector`) (`KismetMathLibrary.Conv_DoubleToVector` 600.0))) (`KismetMathLibrary.ComposeRotators` _returnvalue_rotation (`KismetMathLibrary.MakeRotator` 0.0 0.0 180.0))) false false))
        (:`else`)))))

(event `self.ReceiveTick`
  (params (DeltaSeconds :type "Float (single-precision)"))
  ;[1 1 1] IngameMenu Interaction
  (`self.WidgetInteractionForIngame`))

(event `InputAction|TriggerLeft`
  (params (Key :type "Key Structure"))
  (bind _widgetinteractionleft (`self.WidgetInteractionLeft`))
  (bind _paused (`self.Paused`))
  ;[1 1 1] IngameMenu Interaction
  (:`Pressed`
    (if true
      _
      (elif _paused
        (`WidgetInteractionComponent.PressPointerKey` _widgetinteractionleft "LeftMouseButton"))))
  (:`Released`
    (if true
      _
      (elif _paused
        (`WidgetInteractionComponent.ReleasePointerKey` _widgetinteractionleft "LeftMouseButton")
        (set `self.Paused` false :!label _label_2)))))

(event `InputAction|TriggerRight`
  (params (Key :type "Key Structure"))
  (bind _paused (`self.Paused`))
  (bind _widgetinteractionright (`self.WidgetInteractionRight`))
  ;[1 1 1] IngameMenu Interaction
  (:`Pressed`
    (if true
      _
      (elif _paused
        (`WidgetInteractionComponent.PressPointerKey` _widgetinteractionright "LeftMouseButton"))))
  (:`Released`
    (if true
      _
      (elif _paused
        (`WidgetInteractionComponent.ReleasePointerKey` _widgetinteractionright "LeftMouseButton")
        (goto _label_2)))))

(event `SetupGridPointer`
  ;[1 1 1] HousePlacement
  ;;[1 1 1] Sätter upp overlapp event grejen för pekaren
  (`KismetSystemLibrary.PrintString` "Hello" true true (struct :`G` 0.66 :`B` 1.0 :`A` 1.0) 1000.0)
  (bind _returnvalue (`|SpawnActorFromClass` "/Game/Blueprints/pointer.pointer_C" (`KismetMathLibrary.MakeTransform` (0.0 0.0 -10000.0) (`KismetMathLibrary.MakeRotator` 0.0 0.0) (0.02 0.02 200.0)) "Undefined" "OverrideRootScale" null null))
  (bind _output_get (set `self.Pointer` _returnvalue))
  (`self.K2_AttachToComponent` _output_get (`self.PointerMesh`) "None" "KeepRelative" "KeepRelative" "KeepRelative" true)
  (add `self.OnActorBeginOverlap` _output_get (delegate `OnActorBeginOverlap_Event_0`))
  (add `self.OnActorEndOverlap` _output_get (delegate `OnActorEndOverlap_Event_0`)))

(event `OnActorBeginOverlap_Event_0` :!signature `self.OnActorBeginOverlap`
  (params (OverlappedActor :type "Actor Object Reference") (OtherActor :type "Actor Object Reference"))
  ;[1 1 1] HousePlacement
  ;;[1 1 1] Passivt håller koll på om pekaren pekar på någon ruta och vilken ruta pekaren pekar på(Selectar)
  (set `self.selected` true)
  (if (`KismetStringLibrary.Contains` (`KismetSystemLibrary.GetDisplayName` OtherActor) "block" true)
    (bind _asblock (cast `/Game/Blueprints/block` OtherActor))
    (bind _output_get (set `self.Selected item` _asblock))
    (`PrimitiveComponent.SetMaterial` (`/Game/Blueprints/block.Cube` _output_get) 0 "/Game/Materials/SelectedGridMaterial.SelectedGridMaterial")))

(event `OnActorEndOverlap_Event_0` :!signature `self.OnActorEndOverlap`
  (params (OverlappedActor :type "Actor Object Reference") (OtherActor :type "Actor Object Reference"))
  ;[1 1 1] HousePlacement
  ;;[1 1 1] Passivt håller koll på om pekaren pekar på någon ruta och vilken ruta pekaren pekar på(Selectar)
  (set `self.selected` false) ; Behöver fixa så att den slutar selecta något när man siktar mot luften i framtiden
  (if (`KismetStringLibrary.Contains` (`KismetSystemLibrary.GetDisplayName` OtherActor) "block" true)
    (bind _asblock (cast `/Game/Blueprints/block` OtherActor))
    (`PrimitiveComponent.SetMaterial` (`/Game/Blueprints/block.Cube` _asblock) 0 "/Game/Materials/GridMaterial.GridMaterial")))

(event `InputAction|TriggerRight`
  (params (Key :type "Key Structure"))
  (bind _selected_item (`self.Selected item`))
  (bind _outactors (`self.GetAttachedActors` (`self.Selected item`) true false))
  (bind _output (`|GetArrayItem` _outactors))
  ;[1 1 1] HousePlacement
  ;;[1 1 1] Ser till att A knappen fungerar som toggle
  (:`Pressed`
    (if (`self.Toggle`)
      ;;[0.01338 1 0] Spawnar hus på "Selectade" rutan(här kan du ändra vad du vill spawna och dess transform)
      (if (`self.selected`)
        (bind _returnvalue (`|SpawnActorFromClass` "/Game/Blueprints/house.house_C" (`KismetMathLibrary.MakeTransform` (`self.K2_GetActorLocation` _selected_item) (struct) (0.5 0.5 0.5)) "AlwaysSpawn" "OverrideRootScale" null null))
        (`self.K2_AttachToActor` _returnvalue _selected_item "None" "KeepWorld" "KeepRelative" "KeepWorld" true))
      (else
        ;;[1 1 1] Tar bort saker husen i den "selectade området(ifall det inte finns ett hus så händer inget)
        (if (`self.selected`)
          (if (!= _output null)
            (`self.K2_DestroyActor` _output)
            (`KismetArrayLibrary.Array_Remove` _outactors))))))
  (:`Released`
    (bind _output_get (set `self.Toggle` (!= (stale _output_get) true)))))

(fn `UpdateMission`
  (params (currentMission :type String))
  ;[1 1 1] Updates quest UI Text
)

(fn `UserConstructionScript`)

(fn `WidgetInteractionForIngame`
  (bind _widgetinteractionleft (`self.WidgetInteractionLeft`))
  (bind _widgetinteractionright (`self.WidgetInteractionRight`))
  (bind _returnvalue (`SceneComponent.K2_GetComponentLocation` _widgetinteractionright))
  (bind _returnvalue_2 (`SceneComponent.K2_GetComponentLocation` _widgetinteractionleft))
  (bind (_returnvalue_bblockinghit _returnvalue_binitialoverlap _returnvalue_time _returnvalue_distance _returnvalue_location) (`GameplayStatics.BreakHitResult` (`WidgetInteractionComponent.GetLastHitResult` _widgetinteractionleft)))
  (bind (_returnvalue_bblockinghit_2 _returnvalue_binitialoverlap_2 _returnvalue_time_2 _returnvalue_distance_2 _returnvalue_location_2) (`GameplayStatics.BreakHitResult` (`WidgetInteractionComponent.GetLastHitResult` _widgetinteractionright)))
  (bind _returnvalue_3 (`KismetMathLibrary.GetForwardVector` (`KismetMathLibrary.FindLookAtRotation` _returnvalue_2 _returnvalue_location)))
  (bind _returnvalue_4 (`KismetMathLibrary.GetForwardVector` (`KismetMathLibrary.FindLookAtRotation` _returnvalue _returnvalue_location_2)))
  (`|ExecutionSequence`
    (:`then_0`
      (bind _leftspline (`self.LeftSpline`)
        (:`then`
          (`ActorComponent.K2_DestroyComponent` _leftspline))
        (:`else`
          _))
      (if (`WidgetInteractionComponent.IsOverHitTestVisibleWidget` _widgetinteractionleft)
        (bind _returnvalue_5 (`AddComponent|NODE_AddSplineMeshComponent-0` :`bManualAttachment` true))
        (bind _output_get (set `self.LeftSpline` _returnvalue_5))
        (`SplineMeshComponent.SetStartAndEnd` _output_get _returnvalue_2 _returnvalue_3 _returnvalue_location (* _returnvalue_3 (`KismetMathLibrary.Conv_DoubleToVector` -1.0)) true)))
    (:`then_1`
      (bind _rightspline (`self.RightSpline`)
        (:`then`
          (`ActorComponent.K2_DestroyComponent` _rightspline))
        (:`else`
          _))
      (if (`WidgetInteractionComponent.IsOverHitTestVisibleWidget` _widgetinteractionright)
        (bind _returnvalue_6 (`AddComponent|NODE_AddSplineMeshComponent-1` :`bManualAttachment` true))
        (bind _output_get_2 (set `self.RightSpline` _returnvalue_6))
        (`SplineMeshComponent.SetStartAndEnd` _output_get_2 _returnvalue _returnvalue_4 _returnvalue_location_2 (* _returnvalue_4 (`KismetMathLibrary.Conv_DoubleToVector` -1.0)) true)))))