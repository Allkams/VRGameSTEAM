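; BP_NPC is a template NPC that shows dialogue and completes a player quest when the conversation ends.
; Each Talk call advances through the Dialogue array in a WB_Dialogue widget and flags BP_ThirdPersonCharacter2 as talking.
; When lines run out it removes the widget, marks the player done and calls CompleteQuest once through a DoOnce.
; A recursive random-roam event and a background sound exist but are never triggered here.
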(event `self.ReceiveBeginPlay`
  ;[1 1 1] AI Roam Around (Random roam)
)

(event `Roam`
  ;[1 1 1] AI Roam Around (Random roam)
  (`|AIMoveTo` self (`NavigationSystemV1.K2_GetRandomReachablePointInRadius` (`self.K2_GetActorLocation`) 2000.0 null null) null
    (:`OnSuccess`
      (`self.Roam`))))

(event `/Game/MyContent/Quest_Dialogue/BPI_Dialogue.Talk`
  ;[1 1 1] NPC Dialogue Controller
  (`/Engine/EditorBlueprintResources/StandardMacros.IncrementInt` (`self.talkIndex`)
    (:`  `
      (if (< (`self.talkIndex`) (`KismetArrayLibrary.Array_Length` (`self.dialogue`)))
        (`self.UI`
          (:`then`
            _)
          (:`else`
            (bind _returnvalue (`|CreateWidget` "/Game/MyContent/Quest_Dialogue/WB_Dialogue.WB_Dialogue_C" (`GameplayStatics.GetPlayerController` 0)))
            (bind _output_get (set `self.UI` _returnvalue))
            (`UserWidget.AddToViewport` _output_get 0)))
        (`TextBlock.SetText` (`/Game/MyContent/Quest_Dialogue/WB_Dialogue.TalkText` (`self.UI`)) (`KismetTextLibrary.Conv_StringToText` (`|GetArrayItem` (`self.dialogue`) (`self.talkIndex`))))
        (bind _returnvalue_2 (`GameplayStatics.GetActorOfClass` "/Game/MyContent/Quest_Dialogue/BP_ThirdPersonCharacter2.BP_ThirdPersonCharacter2_C"))
        (set `/Game/MyContent/Quest_Dialogue/BP_ThirdPersonCharacter2.isTalking` true _returnvalue_2)
        (else
          (`Widget.RemoveFromParent` (`self.UI`))
          (bind _returnvalue_3 (`GameplayStatics.GetActorOfClass` "/Game/MyContent/Quest_Dialogue/BP_ThirdPersonCharacter2.BP_ThirdPersonCharacter2_C"))
          (set `/Game/MyContent/Quest_Dialogue/BP_ThirdPersonCharacter2.isTalking` false _returnvalue_3)
          (set `/Game/MyContent/Quest_Dialogue/BP_ThirdPersonCharacter2.isDone` true _returnvalue_3)
          (`/Engine/EditorBlueprintResources/StandardMacros.DoOnce` false
            (:`Completed`
              (`/Game/MyContent/Quest_Dialogue/BP_ThirdPersonCharacter2.CompleteQuest` _returnvalue_3))))))))

(fn `UserConstructionScript`)